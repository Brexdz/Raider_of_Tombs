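; KeyDoorBP is a door that the player opens with the E key once holding the first keycard.
; Overlapping its Box enables input on the actor if the ThirdPersonCharacter's Keycards entry at index 0 is true.
; Pressing E plays the DoorOpen timeline, which drives the KeyDoor component's relative location.
; The logic to disable input and reverse the timeline is unconnected, so the door never closes and input stays enabled.
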(event `self.Box.OnComponentBeginOverlap`
  (params (OverlappedComponent :type "PrimitiveComponent Object Reference") (OtherActor :type "Actor Object Reference") (OtherComp :type "PrimitiveComponent Object Reference") (OtherBodyIndex :type Integer) (bFromSweep :type Boolean) (SweepResult :type "HitResult Structure (by ref)"))
  (bind _asthird_person_character (cast `/Game/ThirdPersonBP/Blueprints/ThirdPersonCharacter` OtherActor))
  (for (_array_element _array_index) (`/Game/ThirdPersonBP/Blueprints/ThirdPersonCharacter.keycards` _asthird_person_character)
    (if (and _array_element (== _array_index 0))
      (`self.EnableInput` (`GameplayStatics.GetPlayerController` 0)))))

(event `Key|E`
  (params (Key :type "Key Structure"))
  (:`Pressed`
    (bind (_direction _dooropen_track) (`Timeline|DoorOpen`)
      (:`Update`
        (`SceneComponent.K2_SetRelativeLocation` (`self.KeyDoor`) _dooropen_track false false)))))

(fn `UserConstructionScript`)