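; Puzzle door Blueprint that swings its static mesh open and closed through DoorOpen and closedoor events.
; BeginPlay caches the mesh's world rotation as the default.
; DoorOpen plays a timeline whose ZAxis track, despite its name, drives a pitch offset combined with that default each update.
; The closedoor event reverses the same timeline.
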(event `self.ReceiveBeginPlay`
  (set `self.defaultrotation` (`SceneComponent.K2_GetComponentRotation` (`self.StaticMeshComponent`))))

(event `DoorOpen`
  (bind (_direction _zaxis) (`Timeline|DoorTimeline` :!label _label)
    (:`Update`
      (`SceneComponent.K2_SetWorldRotation` (`self.StaticMeshComponent`) (`KismetMathLibrary.ComposeRotators` (`KismetMathLibrary.MakeRotator` 0.0 _zaxis) (`self.defaultrotation`)) false false))))

(event `close door`
  (goto _label :!via `Reverse`))

(fn `UserConstructionScript`)