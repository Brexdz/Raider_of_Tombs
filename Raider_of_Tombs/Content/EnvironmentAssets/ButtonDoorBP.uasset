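; Interactive door Blueprint that the player opens and closes with a nearby button.
; An interaction box enables input and opens a Gate while the ThirdPersonCharacter overlaps it.
; Pressing interact plays push and door sounds ahead of the Gate, then a timeline dips the button before a FlipFlop plays or reverses the door-sliding timeline.
; The construction script places the button from its ButtonTransform variable.
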(event `InputAction|InteractBUTTON`
  (params (Key :type "Key Structure"))
  (bind _button_transform_location (`KismetMathLibrary.BreakTransform` (`self.Button Transform`)))
  ;[1 1 1] Hit 1 to open door if player is close enough
  (:`Pressed`
    (`GameplayStatics.PlaySound2D` "/Game/Sounds/ButtonPush.ButtonPush" 1.0 1.0 0.0 null null)
    (`GameplayStatics.PlaySound2D` "/Game/Sounds/DoorOpen.DoorOpen" 1.0 1.0 0.0 null null)
    (`/Engine/EditorBlueprintResources/StandardMacros.Gate` true :!label _label
      (:`Exit`
        ;[1 1 1] push button
        (bind (_direction _button_track) (`Timeline|ButtonPress` :!via `PlayFromStart`)
          (:`Update`
            (`SceneComponent.K2_SetRelativeLocation` (`self.Button`) (`KismetMathLibrary.VLerp` _button_transform_location (- _button_transform_location (0.0 0.0 5.0)) _button_track) false false))
          (:`Finished`
            ;[1 1 1] open and close door
            (`/Engine/EditorBlueprintResources/StandardMacros.FlipFlop`
              (:`A`
                (bind (_direction_2 _dooropen) (`Timeline|Door Timeline` :!label _label_2)
                  (:`Update`
                    (`SceneComponent.K2_SetRelativeLocation` (`self.Door`) _dooropen false false))))
              (:`B`
                (goto _label_2 :!via `Reverse`)))))))))

(event `self.interaction box.OnComponentBeginOverlap`
  (params (OverlappedComponent :type "PrimitiveComponent Object Reference") (OtherActor :type "Actor Object Reference") (OtherComp :type "PrimitiveComponent Object Reference") (OtherBodyIndex :type Integer) (bFromSweep :type Boolean) (SweepResult :type "HitResult Structure (by ref)"))
  ;[1 1 1] Hit 1 to open door if player is close enough
  (cast `/Game/ThirdPersonBP/Blueprints/ThirdPersonCharacter` OtherActor)
  (`self.EnableInput` (`GameplayStatics.GetPlayerController` 0))
  (goto _label :!via `Open`))

(event `self.interaction box.OnComponentEndOverlap`
  (params (OverlappedComponent :type "PrimitiveComponent Object Reference") (OtherActor :type "Actor Object Reference") (OtherComp :type "PrimitiveComponent Object Reference") (OtherBodyIndex :type Integer))
  ;[1 1 1] Hit 1 to open door if player is close enough
  (cast `/Game/ThirdPersonBP/Blueprints/ThirdPersonCharacter` OtherActor)
  (`self.DisableInput` (`GameplayStatics.GetPlayerController` 0))
  (goto _label :!via `Close`))

(fn `UserConstructionScript`
  (`SceneComponent.K2_SetRelativeTransform` (`self.Button`) (`self.Button Transform`) false false))